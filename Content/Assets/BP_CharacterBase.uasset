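; Base character Blueprint that handles weapon switching and exposes the active weapon's idle and walk animations.
; Switching stores a pending weapon and plays a montage, while a separate event stows the current weapon and puts the pending one in hand.
; BeginPlay requests a base weapon after a delay, but AcquireNewWeapon is empty and its spawn-and-attach-to-socket chain is disconnected.
; Incoming damage is only printed.
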(event Custom|AcquireNewWeapon
  (params (WeaponClass :type BP%20Weapon%20Base%20Class%20Reference)))

(event Custom|SwitchActiveWeaponTo
  (params (NewActiveWeapon :type BP%20Weapon%20Base%20Object%20Reference))
  (Variables|Default|SetPendingNextActiveWeapon NewActiveWeapon)
  (Animation|Montage|PlayMontage (Variables|Character|GetMesh) "/Game/Animations/ASM_WeaponSwitch.ASM_WeaponSwitch"))

(event Custom|WeaponSwitchInInventory
  (Utilities|FlowControl|Sequence
    (:then_0
      (Utilities|IsValid (Variables|Default|GetCurrentActiveWeapon)
        (:Is%20Valid
          (Default|WeaponinInventory (Variables|Default|GetCurrentActiveWeapon)))))
    (:then_1
      (bind _output_get (Variables|Default|SetCurrentActiveWeapon (Variables|Default|GetPendingNextActiveWeapon)))
      (Default|WeaponinHand _output_get))))

(event EventBeginPlay
  (Utilities|FlowControl|Delay 3.0)
  (CallFunction|AcquireNewWeapon "/Game/Blueprints/Weapons/BP_WeaponBase.BP_WeaponBase_C"))

(event EventTick
  (params (DeltaSeconds :type Float%20%28single-precision%29)))

(event Collision|EventActorBeginOverlap
  (params (OtherActor :type Actor%20Object%20Reference)))

(event Game|Damage|EventAnyDamage
  (params (Damage :type Float%20%28single-precision%29) (DamageType :type Damage%20Type%20Object%20Reference) (InstigatedBy :type Controller%20Object%20Reference) (DamageCauser :type Actor%20Object%20Reference))
  (Development|PrintString (Utilities|String|ToString(Float) Damage)))

(fn ConstructionScript)

(fn GetActiveWeaponAnims
  (bind _currentactiveweapon (Variables|Default|GetCurrentActiveWeapon))
  (return (Variables|/Game/Blueprints/Weapons/BP_WeaponBase.BP_WeaponBase_C|GetIdleAnim _currentactiveweapon) (Variables|/Game/Blueprints/Weapons/BP_WeaponBase.BP_WeaponBase_C|GetWalkAnim _currentactiveweapon)))