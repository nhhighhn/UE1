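; Melee weapon Blueprint that deals area damage when its CommitAttackAnimNotify event fires.
; The event runs a sphere overlap at the weapon actor's location for Pawn objects, ignoring the owner, and applies BaseDamage to each hit actor with itself as damage causer.
; SphereRadius sets the reach; BeginPlay, overlap and Tick events are unused.
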(event EventBeginPlay)

(event Collision|EventActorBeginOverlap
  (params (OtherActor :type Actor%20Object%20Reference))
  (|CallParentFunction OtherActor) ; This node is disabled and will not be called.\nDrag off pins to build functionality.
)

(event EventTick
  (params (DeltaSeconds :type Float%20%28single-precision%29))
  (|CallParentFunction DeltaSeconds) ; This node is disabled and will not be called.\nDrag off pins to build functionality.
)

(event EventCommitAttackAnimNotify
  (bind _outactors (Collision|SphereOverlapActors (Transformation|GetActorLocation) (Variables|Default|GetSphere%20Radius) (Utilities|Array|MakeArray "ObjectTypeQuery3") 0 (Utilities|Array|MakeArray (Components|GetOwner))))
  (for _array_element _outactors
    (Game|Damage|ApplyDamage _array_element (Variables|Default|GetBase%20Damage) 0 self)))

(fn ConstructionScript
  (|CallParentFunction))